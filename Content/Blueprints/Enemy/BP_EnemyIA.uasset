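; Enemy pawn AI that chases the player once spotted, plays a montage on arrival and dies from damage.
; PawnSensing sets a sight flag that never clears and triggers AIMoveTo, with montage playback gated by CanAttack; Tick halts movement until then.
; Player character overlap with the sphere damages the enemy itself, not the player.
; Damage is scaled and subtracted from printed Health, spawning fire and destroying the actor at zero.
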(event `self.ReceiveTick`
  (params (DeltaSeconds :type "Float (single-precision)"))
  (if (not (`self.IsSeePlayer?`))
    (`MovementComponent.StopMovementImmediately` (`self.CharacterMovement`))))

(event `self.PawnSensing.OnSeePawn`
  (params (Pawn :type "Pawn Object Reference"))
  (set `self.IsSeePlayer?` true)
  (`self.FollowPlayer`))

(event `FollowPlayer`
  (set `self.canAttack?` true)
  (if (`self.IsSeePlayer?`)
    (`|AIMoveTo` self (0.0 0.0 0.0) (`GameplayStatics.GetPlayerCharacter` 0) 70.0
      (:`OnSuccess`
        (if (`self.canAttack?`)
          (set `self.canAttack?` false)
          (bind _returnvalue (`self.PlayAnimMontage` null))
          (`KismetSystemLibrary.Delay` _returnvalue)
          (set `self.canAttack?` true))))
    (else
      (set `self.IsSeePlayer?` false))))

(event `self.Sphere.OnComponentBeginOverlap`
  (params (OverlappedComponent :type "PrimitiveComponent Object Reference") (OtherActor :type "Actor Object Reference") (OtherComp :type "PrimitiveComponent Object Reference") (OtherBodyIndex :type Integer) (bFromSweep :type Boolean) (SweepResult :type "HitResult Structure (by ref)"))
  (cast `/Game/ThirdPerson/Blueprints/BP_ThirdPersonCharacter` OtherActor)
  (`GameplayStatics.ApplyDamage` self 0.5))

(event `self.ReceiveAnyDamage`
  (params (Damage :type "Float (single-precision)") (DamageType :type "DamageType Object Reference") (InstigatedBy :type "Controller Object Reference") (DamageCauser :type "Actor Object Reference"))
  (bind _output_get (set `self.Health` (- (`self.Health`) (* Damage 100.0))))
  (`KismetSystemLibrary.PrintString` (`KismetStringLibrary.Conv_Int64ToString` _output_get) true true (struct :`G` 0.66 :`B` 1.0 :`A` 1.0) 0.5)
  (if (<= (`self.Health`) 0)
    (`GameplayStatics.SpawnEmitterAttached` "/Game/StarterContent/Particles/P_Fire.P_Fire" (`self.CapsuleComponent`))
    (`self.K2_DestroyActor`)))

(fn `UserConstructionScript`)